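; Player character Blueprint that handles walking, mouse look, jumping, sprinting and switching between first- and third-person cameras.
; Axis inputs move along the actor's forward and right vectors, while sprinting swaps max walk speed between walk and sprint values.
; Two custom events toggle the active camera, and both disable controller-yaw rotation and orient-to-movement.
; BeginPlay always starts in third person through a hardwired branch.
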(event `InputAxis|Move Forward / Backward`
  (params (AxisValue :type "Float (single-precision)"))
  ; Movement
  (`self.AddMovementInput` (`self.GetActorForwardVector`) AxisValue))

(event `InputAxis|Move Right / Left`
  (params (AxisValue :type "Float (single-precision)"))
  ; Movement
  (`self.AddMovementInput` (`self.GetActorRightVector`) AxisValue))

(event `InputAxis|Turn Right / Left Mouse`
  (params (AxisValue :type "Float (single-precision)"))
  ; Movement
  (`self.AddControllerYawInput` AxisValue))

(event `InputAxis|Look Up / Down Mouse`
  (params (AxisValue :type "Float (single-precision)"))
  ; Movement
  (`self.AddControllerPitchInput` AxisValue))

(event `InputAction|Jump`
  (params (Key :type "Key Structure"))
  ; Movement
  (:`Pressed`
    (`self.Jump`))
  (:`Released`
    (`self.StopJumping`)))

(event `InputAction|Sprint`
  (params (Key :type "Key Structure"))
  (bind _charactermovement (`self.CharacterMovement`))
  ; Movement
  (:`Pressed`
    (set `self.Is Sprinting` true)
    (set `CharacterMovementComponent.MaxWalkSpeed` (`self.SprintSpeed`) _charactermovement))
  (:`Released`
    (set `self.Is Sprinting` false)
    (set `CharacterMovementComponent.MaxWalkSpeed` (`self.WalkSpeed`) _charactermovement)))

(event `ChangeToFirstperson`
  ; CAM
  (set `self.IsFirstperson` true)
  (`ActorComponent.SetActive` (`self.First_Person_Cam`) true false)
  (`ActorComponent.SetActive` (`self.Third_Person_Cam`) false true)
  (set `self.bUseControllerRotationYaw` false)
  (set `CharacterMovementComponent.bOrientRotationToMovement` false (`self.CharacterMovement`)))

(event `ChangeToThirdperson`
  ; CAM
  (set `self.IsFirstperson` false)
  (`ActorComponent.SetActive` (`self.First_Person_Cam`) false true)
  (`ActorComponent.SetActive` (`self.Third_Person_Cam`) true false)
  (set `self.bUseControllerRotationYaw` false)
  (set `CharacterMovementComponent.bOrientRotationToMovement` false (`self.CharacterMovement`)))

(event `self.ReceiveBeginPlay`
  ; CAM
  (if true
    (`self.ChangeToThirdperson`)
    (else
      (`self.ChangeToFirstperson`))))

(event `InputAction|ToggleCAM`
  (params (Key :type "Key Structure"))
  ; CAM
  (:`Pressed`
    (if (`self.IsFirstperson`)
      (`self.ChangeToThirdperson`)
      (else
        (`self.ChangeToFirstperson`)))))

(fn `UserConstructionScript`)