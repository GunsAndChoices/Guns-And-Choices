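; BP_InventoryManager is an early-stage inventory manager Blueprint for adding items to slots by ItemID.
; AddItemToSlot calls SearchID and, when it reports a match, adds the returned item to an array.
; SearchID loops over an Items array with an empty body, then compares only the final element's ItemID.
; RemoveItemFromSlot, SwapItems, the construction script and the event graph are empty stubs.
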(fn `AddItemToSlot`
  (params (ItemID :type String))
  (bind (_found _item) (`self.SearchID` ItemID))
  (if _found
    (`KismetArrayLibrary.Array_Add` :`NewItem` _item)))

(fn `RemoveItemFromSlot`)

(fn `SearchID`
  (params (ItemID :type String))
  (returns (Found :type Boolean) (Item :type "/Game/Invetar/Item/FItemData Structure"))
  (for _array_element (`.Items_3_858DA8DE487C1790E28832B4F40C67DA` (break `/Game/Invetar/AllItems` (struct)))
    _)
  (if (`KismetStringLibrary.EqualEqual_StrStr` (`.ItemID_17_B9A0DE434B32DC5CDF1371B6F13C446D` (break `/Game/Invetar/Item/FItemData` _array_element)) ItemID)
    (return true _array_element)
    (else
      (return false))))

(fn `SwapItems`)

(fn `UserConstructionScript`)