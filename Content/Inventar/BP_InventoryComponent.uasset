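; Inventory component that holds item data in a content array, apparently for a tile-grid inventory, still unfinished.
; AddAmountToInventory loops over matching stackable items, overwrites their quantity with the amount that fits and tracks the remainder.
; Its follow-up loop for the remainder is empty and its return is never reached.
; TryAddItem is empty, and FindEmptySlot takes a tile size but always reports no slot found.
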(fn `AddAmountToInventory`
  (params (InItemInfo :type "/Game/Inventar/BP_ItemStruct Structure") (InAmount :type Integer))
  (returns (Succes :type Boolean) (RestAmount :type Integer))
  (locals (L_Remaing :type Integer) (InventoryContent :type "Array of /Game/Inventar/S_InventoryItemData Structure") (SpaceinStack :type Integer :default 0))
  (bind (_itemname _itemid _description _icon _wolrdmesh _tilesize _itemtype _slottype _maxstacksize _canstack) (break `/Game/Inventar/BP_ItemStruct` InItemInfo))
  (bind _inventorycontent (`local.InventoryContent`))
  (bind _output_get (set `local.L_Remaing` InAmount))
  (`|ExecutionSequence`
    (:`then_0`
      (if _canstack
        (for (_array_element _array_index) _inventorycontent
          (bind (_itemid_2 _topleftindex _quantity) (break `/Game/Inventar/S_InventoryItemData` _array_element))
          (if (and (`KismetStringLibrary.EqualEqual_StrStr` _itemid_2 _itemid) (<= _quantity _maxstacksize))
            (bind _returnvalue (`KismetMathLibrary.Min` _output_get (- _maxstacksize _quantity)))
            (bind _structout (setmembers `/Game/Inventar/S_InventoryItemData` :`StructRef` _array_element :`Quantity` _returnvalue))
            (`KismetArrayLibrary.Array_Set` _inventorycontent _array_index _structout)
            (set `local.L_Remaing` (- (`local.L_Remaing`) _returnvalue))
            (if (<= _output_get 0)
              (break))))))
    (:`then_1`
      (while (> _output_get 0)
        _))))

(fn `FindEmptySlot`
  (params (InItemTileSize :type "IntPoint Structure"))
  (returns (Found :type Boolean) (GridIndex :type Integer))
  (return false 0))

(fn `TryAddItem`)