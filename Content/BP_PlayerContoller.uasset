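; BP_PlayerContoller is a player controller that toggles the player between first-person and third-person views by switching between two separate characters.
; BeginPlay spawns both characters at the same hardcoded transform, stores them, and possesses the third-person one.
; The ToggleCamera input moves the other character to the current one's location and rotation, possesses it, then sets control rotation and a blended view target.
; The toggle is marked unfinished, and the inactive character is never hidden.
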(event `self.ReceiveBeginPlay`
  (bind _returnvalue (`KismetMathLibrary.MakeTransform` (-750.002563 390.0 226.284607)))
  ;[1 1 1] Init for Camera Toggle
  (bind _returnvalue_2 (`|SpawnActorFromClass` "/Game/FirstPersonBP/Blueprints/FirstPersonCharacter.FirstPersonCharacter_C" _returnvalue "AdjustIfPossibleButAlwaysSpawn" "OverrideRootScale" null null))
  (set `self.character_FPCharater` _returnvalue_2)
  (`KismetSystemLibrary.PrintString` "FP spawned")
  (bind _returnvalue_3 (`|SpawnActorFromClass` "/Game/ThirdPersonBP/Blueprints/ThirdPersonCharacter.ThirdPersonCharacter_C" _returnvalue "AdjustIfPossibleButAlwaysSpawn" "OverrideRootScale" null null))
  (bind _output_get (set `self.character_TPCharater` _returnvalue_3))
  (`KismetSystemLibrary.PrintString` "TP spawned")
  (bind _output_get_2 (set `self.character_CurrentCharacter` _output_get))
  (`self.SetViewTargetWithBlend` (`GameplayStatics.GetPlayerController` 0) _output_get_2 0.0 "VTBlend_Linear" 0.0 false)
  (`self.Possess` (`self.character_CurrentCharacter`)))

(event `InputAction|ToggleCamera`
  (params (Key :type "Key Structure"))
  (bind _character_currentcharacter (`self.character_CurrentCharacter`))
  (bind _character_currentcharacter_2 (`self.character_CurrentCharacter`))
  ;[1 1 1] CameraToggle (Fuck you) [NOT FINISHED]
  (:`Pressed`
    (`/Engine/EditorBlueprintResources/StandardMacros.IsValid` _character_currentcharacter
      (:`Is Valid`
        (bind _output_get (set `self.vector_Location` (`self.K2_GetActorLocation` _character_currentcharacter)))
        (bind _output_get_2 (set `self.rotator_Rotation` (`self.K2_GetActorRotation` _character_currentcharacter)))
        (if (== (`self.character_CurrentCharacter`) (`self.character_TPCharater`))
          (set `self.character_CurrentCharacter` (`self.character_FPCharater`))
          (else
            (set `self.character_CurrentCharacter` (`self.character_TPCharater`))))
        (`/Engine/EditorBlueprintResources/StandardMacros.IsValid` _character_currentcharacter_2
          (:`Is Valid`
            (`self.K2_SetActorLocation` _character_currentcharacter_2 _output_get false false)
            (`self.K2_SetActorRotation` _character_currentcharacter_2 _output_get_2 false)
            (`self.Possess` _character_currentcharacter_2)
            (`self.SetViewTargetWithBlend` _character_currentcharacter_2 2.0)
            (`self.SetControlRotation` _output_get_2))
          (:`Is Not Valid`
            (`KismetSystemLibrary.PrintString` "\"Toggle failed: no target\""))))
      (:`Is Not Valid`
        (`KismetSystemLibrary.PrintString` "No CurrentCharacter")))))

(fn `UserConstructionScript`)